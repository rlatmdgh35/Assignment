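; BP_Door2 is a hinged door that swings away from or toward a side chosen by where the player stands.
; Overlap caches the BP_Player, and Open&Close_Door uses the cross product of the door's right vector and the player's offset to pick the yaw sign.
; A FlipFlop plays or reverses a timeline driving the door's relative yaw.
; The saved sign is reused while the door is moving or open.
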(event `self.ReceiveActorBeginOverlap`
  (params (OtherActor :type "Actor Object Reference"))
  (bind _asbp_player (cast `/Game/Player/BP_Player` OtherActor))
  (set `self.Player` _asbp_player))

(event `Open&Close_Door`
  (if (< 0.0 (.z (`KismetMathLibrary.Cross_VectorVector` (`KismetMathLibrary.GetRightVector` (`SceneComponent.K2_GetComponentRotation` (`self.DefaultSceneRoot`))) (`KismetMathLibrary.MakeVector` (.x (- (`self.K2_GetActorLocation` (`self.Player`)) (`SceneComponent.K2_GetComponentLocation` (`self.DoorFrame`)))) (.y (- (`self.K2_GetActorLocation` (`self.Player`)) (`SceneComponent.K2_GetComponentLocation` (`self.DoorFrame`))))))))
    (set `self.Rotation` 1.0)
    (else
      (set `self.Rotation` -1.0)))
  (if (not (not (or (`self.bClosing`) (`self.bOpen`))))
    (set `self.Rotation` (`self.SaveRotation`)))
  (`/Engine/EditorBlueprintResources/StandardMacros.FlipFlop`
    (:`A`
      (bind (_direction _rotationvalue) (`Timeline|Open / Close_Door` :!label _label)
        (:`Update`
          (bind _output_get (set `self.SaveRotation` (`self.Rotation`)))
          (`SceneComponent.K2_SetRelativeRotation` (`self.Door`) (`KismetMathLibrary.MakeRotator` 0.0 0.0 (* _output_get _rotationvalue)) false false)
          (set `self.bClosing` true))
        (:`Finished`
          (if (`|EnumEquality` _direction "Forward")
            (set `self.bClosing` false)
            (set `self.bOpen` true)
            (else
              (set `self.bClosing` false)
              (set `self.bOpen` false))))))
    (:`B`
      (goto _label :!via `Reverse`))))

(fn `UserConstructionScript`)