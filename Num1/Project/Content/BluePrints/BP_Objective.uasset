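; Objective checkpoint that guides the player through a numbered sequence of markers, then calls Objective on the tagged door after the last one.
; BeginPlay gathers all objectives, hides them and enables the starting one, matched by index as a root component tag.
; Player overlap advances the index and hands collision, decal and arrow visibility to the next marker, tracked on BP_Player.
; Ping-pong timelines bob the arrow vertically.
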(event `Break_Start`
  (goto _label_2 :!via `Break`))

(event `Reverse_Start`
  (bind (_direction _returnlocation) (`Timeline|ArrowLocation_Start` :!via `Reverse` :!label _label)
    (:`Update`
      (`SceneComponent.K2_SetRelativeLocation` (`self.Arrow`) (`KismetMathLibrary.MakeVector` (.x (`SceneComponent.RelativeLocation` (`/Game/BluePrints/BP_Objective.Arrow` (`/Game/Player/BP_Player.Object_Player` (`self.Player`))))) (.y (`SceneComponent.RelativeLocation` (`/Game/BluePrints/BP_Objective.Arrow` (`/Game/Player/BP_Player.Object_Player` (`self.Player`))))) _returnlocation) false false))
    (:`Finished`
      (if (`|EnumEquality` _direction "Forward")
        (`self.Reverse_Start`)
        (else
          (`self.Start_Start`))))))

(event `Start_Start`
  (goto _label))

(event `self.ReceiveBeginPlay`
  (`|ExecutionSequence`
    (:`then_0`
      (bind _outactors (`GameplayStatics.GetAllActorsOfClass` "/Game/Player/BP_Player.BP_Player_C"))
      (set `self.Player` (`|GetArrayItem` _outactors)))
    (:`then_1`
      (bind _outactors_2 (`GameplayStatics.GetAllActorsOfClassWithTag` "/Game/BluePrints/BP_Door.BP_Door_C" "Objective"))
      (set `self.Door` (`|GetArrayItem` _outactors_2)))
    (:`then_2`
      (bind _outactors_3 (`GameplayStatics.GetAllActorsOfClass` "BP_Objective_C"))
      (bind _output_get (set `self.Objective` _outactors_3))
      (for _array_element _output_get
        (set `self.ArrayElement` _array_element)
        (`self.Off_Collision & Visible_Start`))
      (for _array_element_2 (`self.Objective`) :!label _label_2
        (bind _output_get_2 (set `self.ArrayElement` _array_element_2))
        (if (`ActorComponent.ComponentHasTag` (`Actor.RootComponent` _output_get_2) (`KismetStringLibrary.Conv_StringToName` (`KismetStringLibrary.Conv_IntToString` (`self.Index`))))
          (set `/Game/Player/BP_Player.Object_Player` (`self.ArrayElement`) (`self.Player`))
          (`self.Break_Start`)))
      (`self.On_Collision & Visible`)
      (goto _label))))

(event `SetObjective`
  (bind _player (`self.Player`))
  (if (`self.IsValid`)
    (`self.Off_Collision & Visible`)
    (for _array_element (`self.Objective`) :!label _label_3
      (bind _output_get (set `self.ArrayElement` _array_element))
      (if (`ActorComponent.ComponentHasTag` (`Actor.RootComponent` _output_get) (`KismetStringLibrary.Conv_StringToName` (`KismetStringLibrary.Conv_IntToString` (`self.Index`))))
        (set `/Game/Player/BP_Player.Object_Player` (`self.ArrayElement`) _player)
        (set `/Game/Player/BP_Player.Object_Index` (`self.Index`) _player)
        (`self.Break`)))
    (`self.On_Collision & Visible`)
    (bind (_direction _returnlocation) (`Timeline|ArrowLocation` :!label _label_4)
      (:`Update`
        (`SceneComponent.K2_SetRelativeLocation` (`self.Arrow`) (`KismetMathLibrary.MakeVector` (.x (`SceneComponent.RelativeLocation` (`/Game/BluePrints/BP_Objective.Arrow` (`/Game/Player/BP_Player.Object_Player` (`self.Player`))))) (.y (`SceneComponent.RelativeLocation` (`/Game/BluePrints/BP_Objective.Arrow` (`/Game/Player/BP_Player.Object_Player` (`self.Player`))))) _returnlocation) false false))
      (:`Finished`
        (if (`|EnumEquality` _direction "Forward")
          (`self.Reverse`)
          (else
            (`self.Start`)))))
    (else
      (`self.Off_Collision & Visible`)
      (`/Game/BluePrints/BP_Door.Objective` (`self.Door`)))))

(event `Break`
  (goto _label_3 :!via `Break`))

(event `Reverse`
  (goto _label_4 :!via `Reverse`))

(event `Start`
  (goto _label_4))

(event `self.Box.OnComponentBeginOverlap`
  (params (OverlappedComponent :type "PrimitiveComponent Object Reference") (OtherActor :type "Actor Object Reference") (OtherComp :type "PrimitiveComponent Object Reference") (OtherBodyIndex :type Integer) (bFromSweep :type Boolean) (SweepResult :type "HitResult Structure (by ref)"))
  (cast `/Game/Player/BP_Player` OtherActor)
  (`self.Setting`)
  (`self.SetObjective`))

(fn `Add & Reset`
  (returns (ReturnValue :type Boolean))
  (bind _output_get (set `self.Index` (`/Game/Player/BP_Player.Object_Index` (`self.Player`))))
  (bind _result (`/Engine/EditorBlueprintResources/StandardMacros.IncrementInt` _output_get)
    (:`  `
      (return (== _result (`KismetArrayLibrary.Array_Length` (`self.Objective`)))))))

(fn `Off_Collision & Visible`
  (bind _object_player (`/Game/Player/BP_Player.Object_Player` (`self.Player`)))
  (`|ExecutionSequence`
    (:`then_0`
      (`PrimitiveComponent.SetCollisionEnabled` (`/Game/BluePrints/BP_Objective.Box` _object_player) "NoCollision"))
    (:`then_1`
      (`SceneComponent.SetVisibility` (`/Game/BluePrints/BP_Objective.Decal` _object_player) false false)
      (`SceneComponent.SetVisibility` (`/Game/BluePrints/BP_Objective.Arrow` _object_player) false false))))

(fn `Off_Collision & Visible_Start`
  (bind _arrayelement (`self.ArrayElement`))
  (`|ExecutionSequence`
    (:`then_0`
      (`PrimitiveComponent.SetCollisionEnabled` (`/Game/BluePrints/BP_Objective.Box` _arrayelement) "NoCollision"))
    (:`then_1`
      (`SceneComponent.SetVisibility` (`/Game/BluePrints/BP_Objective.Decal` _arrayelement) false false)
      (`SceneComponent.SetVisibility` (`/Game/BluePrints/BP_Objective.Arrow` _arrayelement) false false))))

(fn `On_Collision & Visible`
  (bind _object_player (`/Game/Player/BP_Player.Object_Player` (`self.Player`)))
  (`|ExecutionSequence`
    (:`then_0`
      (`PrimitiveComponent.SetCollisionEnabled` (`/Game/BluePrints/BP_Objective.Box` _object_player) "QueryOnly"))
    (:`then_1`
      (`SceneComponent.SetVisibility` (`/Game/BluePrints/BP_Objective.Decal` _object_player) true false)
      (`SceneComponent.SetVisibility` (`/Game/BluePrints/BP_Objective.Arrow` _object_player) true false))))

(fn `Setting`
  (bind _returnvalue (`self.Add & Reset`))
  (if _returnvalue
    (set `self.IsValid` false)))

(fn `UserConstructionScript`)