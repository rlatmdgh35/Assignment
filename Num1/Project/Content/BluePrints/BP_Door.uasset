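; BP_Door is a sliding double door that opens when a Character overlaps it or the Objective event fires, and closes when the Character leaves.
; DoorTimeLine slides the two doors apart along Y and moves the lock along Z, despite its track being named LockRotation.
; A dynamic material created in the construction script turns the lock's emissive green on opening and red once closing finishes.
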(event `Objective`
  (`MaterialInstanceDynamic.SetVectorParameterValue` (`self.DoorLockMaterial`) "Emissive" (make `LinearColor` 0.0 20.0) :!label _label)
  (bind (_direction _openlocation _lockrotation) (`Timeline|DoorTimeLine` :!label _label_2)
    (:`Update`
      (bind _returnvalue (`KismetMathLibrary.MakeVector` 0.0 _openlocation))
      (`SceneComponent.K2_SetRelativeLocation` (`self.RightDoor`) _returnvalue false false)
      (`SceneComponent.K2_SetRelativeLocation` (`self.LeftDoor`) (* _returnvalue -1.0) false false)
      (`SceneComponent.K2_SetRelativeLocation` (`self.DoorLock`) (`KismetMathLibrary.MakeVector` 0.0 0.0 _lockrotation) false false))
    (:`Finished`
      (if (`|EnumEquality` _direction "Backward")
        (`MaterialInstanceDynamic.SetVectorParameterValue` (`self.DoorLockMaterial`) "Emissive" (make `LinearColor` 20.0))))))

(event `self.ReceiveActorBeginOverlap`
  (params (OtherActor :type "Actor Object Reference"))
  (cast `Character` OtherActor)
  (goto _label))

(event `self.ReceiveActorEndOverlap`
  (params (OtherActor :type "Actor Object Reference"))
  (cast `Character` OtherActor)
  (goto _label_2 :!via `Reverse`))

(fn `UserConstructionScript`
  (bind _returnvalue (`KismetMaterialLibrary.CreateDynamicMaterialInstance` "/Game/Door/MAT_DoorLock_Inst.MAT_DoorLock_Inst"))
  (bind _output_get (set `self.DoorLockMaterial` _returnvalue))
  (`PrimitiveComponent.SetMaterial` (`self.DoorLock`) 0 _output_get))