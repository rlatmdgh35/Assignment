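; Player character Blueprint that handles movement, camera look and interaction with doors and chests.
; Capsule overlaps store the nearby BP_Door2 or BP_Chest with a type, which the E key uses to open or close it.
; Camera-yaw-relative movement and jumping are gated by CanMove, while Sprint and SneakWalk change max walk speed, though SneakWalk has no release reset.
; Key 5 applies damage to the player, and the SettingSpeed call never runs.
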(event `InputAction|Sprint`
  (params (Key :type "Key Structure"))
  (bind _charactermovement (`self.CharacterMovement`))
  (:`Pressed`
    (set `CharacterMovementComponent.MaxWalkSpeed` 600.0 _charactermovement))
  (:`Released`
    (set `CharacterMovementComponent.MaxWalkSpeed` 400.0 _charactermovement)))

(event `InputAction|Jump`
  (params (Key :type "Key Structure"))
  (:`Pressed`
    (if (`self.bCanMove`)
      (`self.Jump`)))
  (:`Released`
    (`self.StopJumping`)))

(event `InputAction|SneakWalk`
  (params (Key :type "Key Structure"))
  (:`Pressed`
    (set `CharacterMovementComponent.MaxWalkSpeed` 200.0 (`self.CharacterMovement`))))

(event `InputAxis|Forward`
  (params (AxisValue :type "Float (single-precision)"))
  (if (`self.bCanMove`)
    (`self.AddMovementInput` (`KismetMathLibrary.GetForwardVector` (`KismetMathLibrary.MakeRotator` 0.0 0.0 (.yaw (`self.GetControlRotation`)))) (`self.GetInputAxisValue`))))

(event `InputAxis|Right`
  (params (AxisValue :type "Float (single-precision)"))
  (if (`self.bCanMove`)
    (`self.AddMovementInput` (`KismetMathLibrary.GetRightVector` (`KismetMathLibrary.MakeRotator` 0.0 0.0 (.yaw (`self.GetControlRotation`)))) (`self.GetInputAxisValue`))))

(event `InputAxis|HorizontalLook`
  (params (AxisValue :type "Float (single-precision)"))
  (`self.AddControllerYawInput` AxisValue))

(event `InputAxis|VerticalLook`
  (params (AxisValue :type "Float (single-precision)"))
  (`self.AddControllerPitchInput` AxisValue))

(event `self.CapsuleComponent.OnComponentBeginOverlap`
  (params (OverlappedComponent :type "PrimitiveComponent Object Reference") (OtherActor :type "Actor Object Reference") (OtherComp :type "PrimitiveComponent Object Reference") (OtherBodyIndex :type Integer) (bFromSweep :type Boolean) (SweepResult :type "HitResult Structure (by ref)"))
  (set `self.CastingObject` OtherActor)
  (`|ExecutionSequence`
    (:`then_0`
      (bind _asbp_door_2 (cast `/Game/BluePrints/BP_Door2` (`self.CastingObject`)))
      (set `self.Door` _asbp_door_2)
      (set `self.bOverlap` true)
      (set `self.Type` "NewEnumerator1"))
    (:`then_1`
      (bind _asbp_chest (cast `/Game/BluePrints/BP_Chest` (`self.CastingObject`)))
      (set `self.Chest` _asbp_chest)
      (set `self.bOverlap` true)
      (set `self.Type` "NewEnumerator2"))))

(event `self.CapsuleComponent.OnComponentEndOverlap`
  (params (OverlappedComponent :type "PrimitiveComponent Object Reference") (OtherActor :type "Actor Object Reference") (OtherComp :type "PrimitiveComponent Object Reference") (OtherBodyIndex :type Integer))
  (set `self.CastingObject` OtherActor)
  (`|ExecutionSequence`
    (:`then_0`
      (cast `/Game/BluePrints/BP_Door2` (`self.CastingObject`))
      (set `self.bOverlap` false)
      (set `self.Type` "NewEnumerator0"))
    (:`then_1`
      (cast `/Game/BluePrints/BP_Chest` (`self.CastingObject`))
      (set `self.bOverlap` false)
      (set `self.Type` "NewEnumerator0"))))

(event `Key|E`
  (params (Key :type "Key Structure"))
  (:`Pressed`
    (if (`self.bOverlap`)
      (switch `/Game/Character/Struct/ECollisionType` (`self.Type`)
        (:`NewEnumerator1`
          (bind _door (`self.Door`)
            (:`then`
              (`/Game/BluePrints/BP_Door2.Open&Close_Door` _door))
            (:`else`)))
        (:`NewEnumerator2`
          (bind _chest (`self.Chest`)
            (:`then`
              (`/Game/BluePrints/BP_Chest.Open&Close_Chest` _chest))
            (:`else`)))))))

(event `Key|Five`
  (params (Key :type "Key Structure"))
  (:`Pressed`
    (`GameplayStatics.ApplyDamage` self 30.0)))

(fn `UserConstructionScript`)