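; BP_Chest is a chest actor whose lid swings open and shut when its Open&Close_Chest event is called.
; The event toggles between OpenChest and CloseChest, ignoring calls while the lid is moving.
; Each branch plays a timeline that pitches ChestTop, then updates the open state and resets the opposite timeline's time.
; Overlapping actors that cast to BP_Player are stored as Player.
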(event `self.ReceiveActorBeginOverlap`
  (params (OtherActor :type "Actor Object Reference"))
  (bind _asbp_player (cast `/Game/Player/BP_Player` OtherActor))
  (set `self.Player` _asbp_player))

(event `Open&Close_Chest`
  (if (`self.bMoving`)
    _
    (elif (not (`self.bOpen`))
      (bind (_direction _rotationvalue) (`Timeline|Open_Chest` :!label _label)
        (:`Update`
          (set `self.bMoving` true)
          (`SceneComponent.K2_SetRelativeRotation` (`self.Chest_Top`) (`KismetMathLibrary.MakeRotator` 0.0 _rotationvalue 180.0) false false))
        (:`Finished`
          (set `self.bOpen` true)
          (`self.SetNewTime_Close`)
          (set `self.bMoving` false)))
      (else
        (bind (_direction_2 _rotationvalue_2) (`Timeline|Close_Chest` :!label _label_2)
          (:`Update`
            (set `self.bMoving` true)
            (`SceneComponent.K2_SetRelativeRotation` (`self.Chest_Top`) (`KismetMathLibrary.MakeRotator` 0.0 _rotationvalue_2 180.0) false false))
          (:`Finished`
            (set `self.bOpen` false)
            (`self.SetNewTime_Open`)
            (set `self.bMoving` false)))))))

(event `SetNewTime_Open`
  (goto _label :!via `SetNewTime`))

(event `SetNewTime_Close`
  (goto _label_2 :!via `SetNewTime`))

(fn `UserConstructionScript`)